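; AI controller for the robot walker, which collects garbage, carries it to the depot and chases a nearby garbage-carrying player while empty-handed.
; Hand-component grab and deposit events switch the target between depot and garbage found by sphere overlap, or a random navigable point.
; Tick polls for arrival, stalls and chase conditions, rerouting after a delay when arrived or stopped.
; Movement uses SimpleMoveTo calls instead of a behavior tree.
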(event `self.ReceiveBeginPlay`
  (`self.PickEmptyMoveTarget`)
  (add `/Game/Garbage/BP_GarbageHandComponent.HandChanged` (`/Game/Robotics/Walker/BP_RobotWalkerChar.BP_GarbageHandComponent` (cast `/Game/Robotics/Walker/BP_RobotWalkerChar` (`self.K2_GetPawn`) :!pure true)) (delegate `HandChanged_Event_0`)))

(event `HandChanged_Event_0`
  (params (NumChanged :type Integer) (Reason :type "/Game/Garbage/EHandChangeReason Enum" :default "NewEnumerator0"))
  (switch `/Game/Garbage/EHandChangeReason` Reason
    (:`NewEnumerator1`
      (`self.PickDepotMoveTarget`) ; just picked up garbage
    )
    (:`NewEnumerator2`
      (`self.PickEmptyMoveTarget`) ; just deposited
    )))

(event `PickDepotMoveTarget`
  (bind _returnvalue (`GameplayStatics.GetActorOfClass` "/Game/Garbage/BP_RobotGarbageDepot.BP_RobotGarbageDepot_C"))
  (`self.MoveTo` (`SceneComponent.K2_GetComponentLocation` (`/Game/Garbage/BP_RobotGarbageDepot.DepositPoint` _returnvalue))))

(event `PickEmptyMoveTarget`
  (bind _searchradius (`self.SearchRadius`))
  (bind _returnvalue (`self.K2_GetActorLocation` (`self.K2_GetPawn`)))
  (bind (_outactors _returnvalue_2) (`KismetSystemLibrary.SphereOverlapActors` _returnvalue _searchradius (`|MakeArray` "ObjectTypeQuery2" :!type "EObjectTypeQuery Enum") "/Game/Garbage/BP_PickableGarbage.BP_PickableGarbage_C")) ; go to nearby garbage
  (if _returnvalue_2
    (`self.MoveTo` (`self.K2_GetActorLocation` (`|GetArrayItem` _outactors)))
    (else
      (bind _randomlocation (`NavigationSystemV1.K2_GetRandomLocationInNavigableRadius` _returnvalue _searchradius null null)) ; otherwise go to some random point
      (`self.MoveTo` _randomlocation))))

(event `self.ReceiveTick`
  (params (DeltaSeconds :type "Float (single-precision)"))
  (bind _returnvalue (`self.K2_GetPawn`))
  (if (== (- (`self.K2_GetActorLocation` _returnvalue) (`KismetMathLibrary.MakeVector` 0.0 0.0 (`CapsuleComponent.CapsuleHalfHeight` (`Character.CapsuleComponent` (cast `Character` _returnvalue :!pure true))))) (`self.MoveTarget`) :`ErrorTolerance` 30.0)
    (`KismetSystemLibrary.Delay` 2.0 :!label _label)
    (if (`self.IsEmptyHanded`)
      (`self.RerouteEmptyHanded`)
      (else
        (`self.PickDepotMoveTarget`)))
    (elif (== (`self.GetVelocity` (`self.K2_GetPawn`)) (0.0 0.0 0.0))
      (goto _label)
      (else
        (bind (_returnvalue_2 _player) (`self.ShouldChasePlayer`))
        (if _returnvalue_2
          (`self.MoveToPlayer` _player)
          (elif (`self.WasChasingPlayer`)
            (set `self.WasChasingPlayer` false)
            (`self.PickEmptyMoveTarget`)))))))

(fn `CancelMoveTo`
  (`self.MoveTo` (`self.K2_GetActorLocation` (`self.K2_GetPawn`))))

(fn `IsEmptyHanded`
  (returns (ReturnValue :type Boolean))
  (return (== (`KismetArrayLibrary.Array_Length` (`/Game/Garbage/BP_GarbageHandComponent.GarbageHeld` (`self.GetComponentByClass` (`self.K2_GetPawn`) "/Game/Garbage/BP_GarbageHandComponent.BP_GarbageHandComponent_C"))) 0)))

(fn `MoveTo`
  (params (Target :type "Vector Structure"))
  (bind _output_get (set `self.MoveTarget` Target))
  (`AIBlueprintHelperLibrary.SimpleMoveToLocation` self _output_get))

(fn `MoveToPlayer`
  (params (Player :type "Actor Object Reference"))
  (`AIBlueprintHelperLibrary.SimpleMoveToActor` self Player)
  (set `self.MoveTarget` (0.0 0.0 -10000.0))
  (set `self.WasChasingPlayer` true))

(fn `RerouteEmptyHanded`
  (bind _returnvalue (`self.TryGetPlayerInRange`))
  (`/Engine/EditorBlueprintResources/StandardMacros.IsValid` _returnvalue
    (:`Is Valid`
      (`self.MoveToPlayer` _returnvalue))
    (:`Is Not Valid`
      (`self.PickEmptyMoveTarget`))))

(fn `ShouldChasePlayer`
  (returns (ReturnValue :type Boolean) (Player :type "/Game/FirstPersonBP/Blueprints/FirstPersonCharacter Object Reference"))
  (bind _returnvalue (`self.TryGetPlayerInRange`))
  (`/Engine/EditorBlueprintResources/StandardMacros.IsValid` _returnvalue
    (:`Is Valid`
      (return (and (!= (`KismetArrayLibrary.Array_Length` (`/Game/Garbage/BP_GarbageHandComponent.GarbageHeld` (`self.GetComponentByClass` _returnvalue "/Game/Garbage/BP_GarbageHandComponent.BP_GarbageHandComponent_C"))) 0) (== (`KismetArrayLibrary.Array_Length` (`/Game/Garbage/BP_GarbageHandComponent.GarbageHeld` (`self.GetComponentByClass` (`self.K2_GetPawn`) "/Game/Garbage/BP_GarbageHandComponent.BP_GarbageHandComponent_C"))) 0)) _returnvalue))))

(fn `TryGetPlayerInRange`
  (returns (ReturnValue :type "/Game/FirstPersonBP/Blueprints/FirstPersonCharacter Object Reference"))
  (bind (_outactors _returnvalue) (`KismetSystemLibrary.SphereOverlapActors` (`self.K2_GetActorLocation` (`self.K2_GetPawn`)) 1000.0 (`|MakeArray` "ObjectTypeQuery2" :!type "EObjectTypeQuery Enum") "/Game/FirstPersonBP/Blueprints/FirstPersonCharacter.FirstPersonCharacter_C"))
  (if _returnvalue
    (return (cast `/Game/FirstPersonBP/Blueprints/FirstPersonCharacter` (`|GetArrayItem` _outactors) :!pure true))))

(fn `UserConstructionScript`)