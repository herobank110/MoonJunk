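; AI controller for a garbage-collecting robot drone that ferries pickable garbage to the depot and chases nearby players carrying garbage.
; Hand-change events switch targets between depot and garbage, falling back to random navigable points.
; Tick moves the pawn by direct unswept offsets without pathfinding, keeping its height or clamping it when chasing.
; A delayed reroute follows arrival or zero velocity, favoring any nearby player when empty-handed.
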(event `self.ReceiveBeginPlay`
  (`self.PickEmptyMoveTarget`)
  (add `/Game/Garbage/BP_GarbageHandComponent.HandChanged` (`/Game/Robotics/Drone/BP_RobotDronePawn.BP_GarbageHandComponent` (cast `/Game/Robotics/Drone/BP_RobotDronePawn` (`self.K2_GetPawn`) :!pure true)) (delegate `HandChanged_Event_0`)))

(event `HandChanged_Event_0`
  (params (NumChanged :type Integer) (Reason :type "/Game/Garbage/EHandChangeReason Enum" :default "NewEnumerator0"))
  (switch `/Game/Garbage/EHandChangeReason` Reason
    (:`NewEnumerator1`
      (`self.PickDepotMoveTarget`) ; just picked up garbage
    )
    (:`NewEnumerator2`
      (`self.PickEmptyMoveTarget`) ; just deposited
    )))

(event `PickDepotMoveTarget`
  (bind _returnvalue (`GameplayStatics.GetActorOfClass` "/Game/Garbage/BP_RobotGarbageDepot.BP_RobotGarbageDepot_C"))
  (`self.MoveTo` (`self.Heightify` (`SceneComponent.K2_GetComponentLocation` (`/Game/Garbage/BP_RobotGarbageDepot.DepositPoint` _returnvalue)))))

(event `PickEmptyMoveTarget`
  (bind _searchradius (`self.SearchRadius`))
  (bind _returnvalue (`self.K2_GetActorLocation` (`self.K2_GetPawn`)))
  (bind (_outactors _returnvalue_2) (`KismetSystemLibrary.SphereOverlapActors` _returnvalue _searchradius (`|MakeArray` "ObjectTypeQuery2" :!type "EObjectTypeQuery Enum") "/Game/Garbage/BP_PickableGarbage.BP_PickableGarbage_C")) ; go to nearby garbage
  (if _returnvalue_2
    (`self.MoveTo` (`self.Heightify` (`self.K2_GetActorLocation` (`|GetArrayItem` _outactors))))
    (else
      (bind _randomlocation (`NavigationSystemV1.K2_GetRandomLocationInNavigableRadius` _returnvalue _searchradius null null)) ; otherwise go to some random point
      (`self.MoveTo` (`self.Heightify` _randomlocation)))))

(event `self.ReceiveTick`
  (params (DeltaSeconds :type "Float (single-precision)"))
  (`self.TickMovement` DeltaSeconds)
  (if (or (== (`self.K2_GetActorLocation` (`self.K2_GetPawn`)) (`self.RealMoveTarget`) :`ErrorTolerance` 30.0) (== (`self.GetVelocity` (`self.K2_GetPawn`)) (0.0 0.0 0.0)))
    (`KismetSystemLibrary.Delay` 2.0)
    (if (`self.IsEmptyHanded`)
      (`self.RerouteEmptyHanded`)
      (else
        (`self.PickDepotMoveTarget`)))
    (else
      (bind (_returnvalue _player) (`self.ShouldChasePlayer`))
      (if _returnvalue
        (`self.MoveToPlayer` _player)
        (elif (`self.WasChasingPlayer`)
          (set `self.WasChasingPlayer` false)
          (`self.PickEmptyMoveTarget`))))))

(fn `Heightify`
  (params (InVec :type "Vector Structure"))
  (returns (ReturnValue :type "Vector Structure"))
  (return (`KismetMathLibrary.MakeVector` (.x InVec) (.y InVec) (.z (`self.K2_GetActorLocation` (`self.K2_GetPawn`))))))

(fn `HeightifyClamp`
  (params (InVec :type "Vector Structure"))
  (returns (ReturnValue :type "Vector Structure"))
  (bind (_lowerbound _upperbound) (break `FloatRange` (`self.HeightRange`)))
  (return (`KismetMathLibrary.MakeVector` (.x InVec) (.y InVec) (`KismetMathLibrary.FClamp` (.z InVec) (`.Value` (break `FloatRangeBound` _lowerbound)) (`.Value` (break `FloatRangeBound` _upperbound))))))

(fn `IsEmptyHanded`
  (returns (ReturnValue :type Boolean))
  (return (== (`KismetArrayLibrary.Array_Length` (`/Game/Garbage/BP_GarbageHandComponent.GarbageHeld` (`self.GetComponentByClass` (`self.K2_GetPawn`) "/Game/Garbage/BP_GarbageHandComponent.BP_GarbageHandComponent_C"))) 0)))

(fn `MoveTo`
  (params (Target :type "Vector Structure"))
  (set `self.MoveTarget` Target)
  (set `self.MoveTargetActor` null) ; clear
)

(fn `MoveToPlayer`
  (params (Player :type "Actor Object Reference"))
  (set `self.MoveTargetActor` Player)
  (set `self.MoveTarget` (0.0 0.0 -10000.0))
  (set `self.WasChasingPlayer` true))

(fn `RealMoveTarget`
  (returns (ReturnValue :type "Vector Structure"))
  (bind _movetargetactor (`self.MoveTargetActor`)
    (:`then`
      (return (`self.HeightifyClamp` (`self.K2_GetActorLocation` _movetargetactor))))
    (:`else`
      (return (`self.MoveTarget`)))))

(fn `RerouteEmptyHanded`
  (bind _returnvalue (`self.TryGetPlayerInRange`))
  (`/Engine/EditorBlueprintResources/StandardMacros.IsValid` _returnvalue
    (:`Is Valid`
      (`self.MoveToPlayer` _returnvalue))
    (:`Is Not Valid`
      (`self.PickEmptyMoveTarget`))))

(fn `ShouldChasePlayer`
  (returns (ReturnValue :type Boolean) (Player :type "/Game/FirstPersonBP/Blueprints/FirstPersonCharacter Object Reference"))
  (bind _returnvalue (`self.TryGetPlayerInRange`))
  (`/Engine/EditorBlueprintResources/StandardMacros.IsValid` _returnvalue
    (:`Is Valid`
      (return (and (!= (`KismetArrayLibrary.Array_Length` (`/Game/Garbage/BP_GarbageHandComponent.GarbageHeld` (`self.GetComponentByClass` _returnvalue "/Game/Garbage/BP_GarbageHandComponent.BP_GarbageHandComponent_C"))) 0) (== (`KismetArrayLibrary.Array_Length` (`/Game/Garbage/BP_GarbageHandComponent.GarbageHeld` (`self.GetComponentByClass` (`self.K2_GetPawn`) "/Game/Garbage/BP_GarbageHandComponent.BP_GarbageHandComponent_C"))) 0)) _returnvalue))))

(fn `TickMovement`
  (params (DeltaTime :type "Float (double-precision)"))
  (bind _returnvalue (`self.RealMoveTarget`))
  (bind _returnvalue_2 (`self.K2_GetPawn`))
  (bind _returnvalue_3 (`self.K2_GetActorLocation` _returnvalue_2))
  (if (!= _returnvalue _returnvalue_3 :`ErrorTolerance` 50.0)
    (`self.K2_AddActorWorldOffset` _returnvalue_2 (* (`KismetMathLibrary.Normal` (- _returnvalue _returnvalue_3)) (* (`self.MoveSpeed`) DeltaTime)) false false)
    (`self.K2_SetActorRotation` _returnvalue_2 (`KismetMathLibrary.MakeRotator` (.roll (`KismetMathLibrary.FindLookAtRotation` _returnvalue_3 _returnvalue)) (`KismetMathLibrary.FClamp` (.pitch (`KismetMathLibrary.FindLookAtRotation` _returnvalue_3 _returnvalue)) -30.0 30.0) (.yaw (`KismetMathLibrary.FindLookAtRotation` _returnvalue_3 _returnvalue))) false)))

(fn `TryGetPlayerInRange`
  (returns (ReturnValue :type "/Game/FirstPersonBP/Blueprints/FirstPersonCharacter Object Reference"))
  (bind (_outactors _returnvalue) (`KismetSystemLibrary.SphereOverlapActors` (`self.K2_GetActorLocation` (`self.K2_GetPawn`)) 1000.0 (`|MakeArray` "ObjectTypeQuery2" :!type "EObjectTypeQuery Enum") "/Game/FirstPersonBP/Blueprints/FirstPersonCharacter.FirstPersonCharacter_C"))
  (if _returnvalue
    (return (cast `/Game/FirstPersonBP/Blueprints/FirstPersonCharacter` (`|GetArrayItem` _outactors) :!pure true))))

(fn `UserConstructionScript`)