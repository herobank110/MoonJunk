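; Scene component that acts as a hand for carrying a stack of garbage up to a capacity.
; Grabbing destroys the pickup and spawns a BP_HeldGarbage attached to the component, offset along X by its index.
; Snatch moves the last item from another hand into this one, and Deposit destroys everything held.
; All three actions report count changes through HandChanged, with Snatch notifying both hands.
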(event `GrabHold`
  (params (Garbage :type "/Game/Garbage/BP_PickableGarbage Object Reference"))
  (if (`self.HasRoomForMore`)
    (`self.ConvertToHeldObject` Garbage)
    (`self.HandChanged` 1)))

(event `Deposit`
  (bind _garbageheld (`self.GarbageHeld`))
  (bind _returnvalue (`KismetArrayLibrary.Array_Length` _garbageheld))
  (if (not (== _returnvalue 0))
    (`self.HandChanged` (- 0 _returnvalue))
    (`Actor.K2_DestroyActor` _garbageheld)
    (`KismetArrayLibrary.Array_Clear` _garbageheld)))

(event `Snatch`
  (params (Victim :type "/Game/Garbage/BP_GarbageHandComponent Object Reference"))
  (bind _garbageheld (`/Game/Garbage/BP_GarbageHandComponent.GarbageHeld` Victim))
  (bind _returnvalue (`KismetArrayLibrary.Array_Length` _garbageheld))
  (bind _returnvalue_2 (- _returnvalue 1))
  (if (`self.HasRoomForMore`)
    (if (!= _returnvalue 0)
      (`self.TransferToOwnHand` (`|GetArrayItem` _garbageheld _returnvalue_2))
      (`self.HandChanged` 1)
      (`KismetArrayLibrary.Array_Remove` _garbageheld _returnvalue_2)
      (`self.HandChanged` Victim -1))))

(fn `ConvertToHeldObject`
  (params (Pickable :type "/Game/Garbage/BP_PickableGarbage Object Reference"))
  (`Actor.K2_DestroyActor` Pickable) ; garbage pick up able no longer needed
  (bind _returnvalue (`|SpawnActorFromClass` "/Game/Garbage/BP_HeldGarbage.BP_HeldGarbage_C" (`KismetMathLibrary.MakeTransform` (0.0 0.0 0.0)) "Undefined" "OverrideRootScale" null null))
  (`KismetArrayLibrary.Array_Add` (`self.GarbageHeld`) _returnvalue)
  (`Actor.K2_AttachToComponent` _returnvalue self "None" "SnapToTarget" "SnapToTarget" "KeepRelative" true) ; grab hold of the garbage
  (`Actor.K2_AddActorLocalOffset` _returnvalue (`self.HeldObjectOffset` (- (`KismetArrayLibrary.Array_Length` (`self.GarbageHeld`)) 1)) false false))

(fn `HasRoomForMore`
  (returns (ReturnValue :type Boolean))
  (return (< (`KismetArrayLibrary.Array_Length` (`self.GarbageHeld`)) (`self.GarbageCapacity`))))

(fn `HeldObjectOffset`
  (params (Index :type Integer))
  (returns (ReturnValue :type "Vector Structure"))
  (return (`KismetMathLibrary.MakeVector` (* Index 25.0))))

(fn `TransferToOwnHand`
  (params (Held :type "/Game/Garbage/BP_HeldGarbage Object Reference (by ref)"))
  (`KismetArrayLibrary.Array_Add` (`self.GarbageHeld`) Held)
  (`Actor.K2_AttachToComponent` Held self "None" "SnapToTarget" "SnapToTarget" "KeepRelative" true)
  (`Actor.K2_AddActorLocalOffset` Held (`self.HeldObjectOffset` (- (`KismetArrayLibrary.Array_Length` (`self.GarbageHeld`)) 1)) false false))