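; Round manager for the Moon Junk match, where the player competes with robots to collect garbage.
; Each round destroys walker and drone robots, triggers spawn zones by round number, sets the game mode timer from per-round arrays and zeroes player points.
; A delayed Tick polls until no pickable or held garbage remains, then a DoOnce-guarded step shows the player-versus-robots score widget and starts the next round after a pause.
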(event `self.ReceiveBeginPlay`
  (`self.NextRound`))

(event `NextRound`
  (`/Engine/EditorBlueprintResources/StandardMacros.IncrementInt` (`self.CurrentRound`)
    (:`  `
      (`self.KillRobots`)
      (`self.RespawnRoundObjects`)
      (`self.ResetCountdown`)
      (bind _outactors (`GameplayStatics.GetAllActorsOfClass` "/Game/Garbage/BP_PickableGarbage.BP_PickableGarbage_C"))
      (bind _output_get (set `self.TotalGarbage` (`KismetArrayLibrary.Array_Length` _outactors)))
      (`KismetSystemLibrary.PrintString` (`KismetStringLibrary.Concat_StrStr` "Spawned " (`KismetStringLibrary.Conv_IntToString` _output_get) " garbage pickup"))
      (set `/Game/FirstPersonBP/Blueprints/FirstPersonCharacter.Point` 0 (cast `/Game/FirstPersonBP/Blueprints/FirstPersonCharacter` (`GameplayStatics.GetPlayerCharacter` 0) :!pure true)))))

(event `self.ReceiveTick`
  (params (DeltaSeconds :type "Float (single-precision)"))
  (bind _point (`/Game/FirstPersonBP/Blueprints/FirstPersonCharacter.Point` (cast `/Game/FirstPersonBP/Blueprints/FirstPersonCharacter` (`GameplayStatics.GetPlayerCharacter` 0) :!pure true)))
  (`KismetSystemLibrary.Delay` 0.2)
  (if (`self.CanEndRound`)
    (`/Engine/EditorBlueprintResources/StandardMacros.DoOnce` false :!label _label
      (:`Completed`
        (bind _returnvalue (`|CreateWidget` "/Game/BetweenLevels/Different.Different_C" null (- (`self.TotalGarbage`) _point) _point))
        (`UserWidget.AddToViewport` _returnvalue 0)
        (`KismetSystemLibrary.Delay` 5.0) ; ensure this matches Different
        (`self.NextRound`)
        (goto _label :!via `Reset`)))))

(fn `CanEndRound`
  (returns (ReturnValue :type Boolean))
  ;[1 1 1] no more garbage waiting to be picked up
  (bind _outactors (`GameplayStatics.GetAllActorsOfClass` "/Game/Garbage/BP_PickableGarbage.BP_PickableGarbage_C"))
  ;[1 1 1] no garbage being held by player or robot
  (bind _outactors_2 (`GameplayStatics.GetAllActorsOfClass` "/Game/Garbage/BP_HeldGarbage.BP_HeldGarbage_C"))
  (return (and (== (`KismetArrayLibrary.Array_Length` _outactors) 0) (== (`KismetArrayLibrary.Array_Length` _outactors_2) 0))))

(fn `KillRobots`
  (bind _outactors (`GameplayStatics.GetAllActorsOfClass` "/Game/Robotics/Walker/BP_RobotWalkerChar.BP_RobotWalkerChar_C"))
  (`self.K2_DestroyActor` _outactors)
  (bind _outactors_2 (`GameplayStatics.GetAllActorsOfClass` "/Game/Robotics/Drone/BP_RobotDronePawn.BP_RobotDronePawn_C"))
  (`self.K2_DestroyActor` _outactors_2))

(fn `ResetCountdown`
  (bind _currentround (`self.CurrentRound`))
  (bind _asfirst_person_game_mode (cast `/Game/FirstPersonBP/Blueprints/FirstPersonGameMode` (`GameplayStatics.GetGameMode`)))
  (set `/Game/FirstPersonBP/Blueprints/FirstPersonGameMode.TimeMin` (`/Game/MatchGameplay/BP_MatchGameplayMacroLib.GetBounded` (`self.TimeMins`) _currentround) _asfirst_person_game_mode)
  (set `/Game/FirstPersonBP/Blueprints/FirstPersonGameMode.TimeSec` (`/Game/MatchGameplay/BP_MatchGameplayMacroLib.GetBounded` (`self.TimeSecs`) _currentround) _asfirst_person_game_mode))

(fn `RespawnRoundObjects`
  (bind _outactors (`GameplayStatics.GetAllActorsOfClass` "/Game/MatchGameplay/BP_SpawnZone.BP_SpawnZone_C"))
  (for _array_element _outactors
    (`/Game/MatchGameplay/BP_SpawnZone.Spawn` _array_element (`self.CurrentRound`))))

(fn `UserConstructionScript`)