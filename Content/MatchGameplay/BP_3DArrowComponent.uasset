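; BP_3DArrowComponent is a component that adds an arrow to its owner and rotates it to point at a target location or actor.
; BeginPlay creates and styles an ArrowComponent at runtime and attaches it to itself, visible in game.
; Setting a target enables Tick, which aims the arrow from the owner's position, preferring a valid actor over the stored location.
; Clearing disables Tick; both setting and clearing hide the arrow.
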(event `self.ReceiveBeginPlay`
  (bind _returnvalue (`|AddComponentByClass` :`self` (`self.GetOwner`) :`Class` "/Script/Engine.ArrowComponent"))
  (bind _output_get (set `self.Mesh` _returnvalue))
  (`self.SetHiddenInGame` _output_get false false)
  (`ArrowComponent.SetArrowColor` _output_get (struct :`R` 0.4375 :`G` 0.374016 :`B` 0.134312 :`A` 1.0))
  (set `ArrowComponent.ArrowLength` 30.0 _output_get)
  (set `ArrowComponent.ArrowSize` 0.5 _output_get)
  (`self.K2_AttachToComponent` _output_get self "None" "SnapToTarget" "SnapToTarget" "KeepRelative" true))

(event `SetTargetLocation`
  (params (TargetLocation :type "Vector Structure"))
  (set `self.TargetLocation` TargetLocation)
  (set `self.TargetActor` null)
  (`self.SetHiddenInGame` (`self.Mesh`) true false :!label _label)
  (`self.SetComponentTickEnabled` true))

(event `SetTargetActor`
  (params (TargetActor :type "Actor Object Reference"))
  (set `self.TargetActor` TargetActor)
  (goto _label))

(event `ClearTargetLocation`
  (`self.SetComponentTickEnabled` false)
  (`self.SetHiddenInGame` (`self.Mesh`) true false))

(event `self.ReceiveTick`
  (params (DeltaSeconds :type "Float (single-precision)"))
  (`self.K2_SetWorldRotation` (`self.Mesh`) (`KismetMathLibrary.FindLookAtRotation` (`Actor.K2_GetActorLocation` (`self.GetOwner`)) (`self.RealTargetLocation`)) false false))

(fn `RealTargetLocation`
  (returns (ReturnValue :type "Vector Structure"))
  (bind _targetactor (`self.TargetActor`)
    (:`then`
      (return (`Actor.K2_GetActorLocation` _targetactor)))
    (:`else`
      (return (`self.TargetLocation`)))))